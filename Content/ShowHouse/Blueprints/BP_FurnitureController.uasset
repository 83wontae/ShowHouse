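; BP_FurnitureController is a laser-pointer tool for placing, deleting, moving and recoloring furniture in the show house.
; A looping timer traces from WidgetInteraction, updating the Niagara laser and aligning a preview mesh to the hit normal plus yaw offset.
; EventTrigger dispatches presses by mode: spawn BP_Furniture, destroy it, attach it to the preview until release, or spawn a palette.
; The preview mesh cycles through DT_Furniture and shows only in Create mode, off widgets.
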(event EventBeginPlay
  (Transformation|AttachComponentToComponent (Variables|Default|GetWidgetInteraction) "None" "KeepRelative" "KeepRelative" "KeepWorld" true)
  (Utilities|Time|SetTimerbyFunctionName 0 "UpdateLineTrace" 0.02 true))

(fn ConstructionScript)

(fn UpdateLineTrace
  (bind _widgetinteraction (Variables|Default|GetWidgetInteraction))
  (bind _ns_menulaser (Variables|Default|GetNS_MenuLaser))
  (bind _ns_menulaser_2 (Variables|Default|GetNS_MenuLaser))
  (bind _returnvalue (Transformation|GetWorldLocation _widgetinteraction))
  (bind _returnvalue_2 (Math|Vector|GetForwardVector _widgetinteraction))
  (bind _interactiondistance (Variables|/Script/UMG.WidgetInteractionComponent|GetInteractionDistance _widgetinteraction))
  (bind _returnvalue_3 (* _returnvalue_2 _interactiondistance))
  (bind _returnvalue_4 (+ _returnvalue _returnvalue_3))
  (Utilities|FlowControl|Sequence
    (:then_0
      (LocalVariables|SetStartLoc _returnvalue)
      (LocalVariables|SetEndLoc _returnvalue_4)
      (bind (_outhit _returnvalue_5) (Collision|LineTraceForObjects _returnvalue _returnvalue_4 (Utilities|Array|MakeArray "ObjectTypeQuery1" "ObjectTypeQuery2") false 0 "None"))
      (if _returnvalue_5
        (Class|NiagaraDataInterfaceArrayFunctionLibrary|SetNiagaraArrayVectorValue _ns_menulaser_2 "User.PointArray" 0 (LocalVariables|GetStartLoc) false) ; MenuLaser start location
        (bind _output_get (LocalVariables|SetEndLoc (.Location (Collision|BreakHitResult _outhit))))
        (Class|NiagaraDataInterfaceArrayFunctionLibrary|SetNiagaraArrayVectorValue _ns_menulaser_2 "User.PointArray" 1 _output_get false) ; MenuLaser end location
        (LocalVariables|SetHitNormal (.ImpactNormal (Collision|BreakHitResult _outhit)))
        (LocalVariables|SetHitComponent (.HitComponent (Collision|BreakHitResult _outhit)))
        (else
          (Class|NiagaraDataInterfaceArrayFunctionLibrary|SetNiagaraArrayVectorValue _ns_menulaser "User.PointArray" 0 (LocalVariables|GetStartLoc) false) ; MenuLaser start location
          (Class|NiagaraDataInterfaceArrayFunctionLibrary|SetNiagaraArrayVectorValue _ns_menulaser "User.PointArray" 1 (LocalVariables|GetEndLoc) false) ; MenuLaser end location
        )))
    (:then_1
      (Transformation|SetWorldLocationAndRotation (Variables|Default|GetFurnitureMesh) (LocalVariables|GetEndLoc) (Math|Rotator|CombineRotators (Math|Rotator|MakeRotfromZX (LocalVariables|GetHitNormal) (* (LocalVariables|GetHitNormal) -1.0)) (Math|Vector|RotatorfromAxisandAngle (LocalVariables|GetHitNormal) (Variables|Default|GetOffsetRotationZ))) false false)
      (if (CallFunction|IsShowFurniture (LocalVariables|GetHitComponent))
        (Rendering|SetVisibility (Variables|Default|GetFurnitureMesh) true false)
        (else
          (Rendering|SetVisibility (Variables|Default|GetFurnitureMesh) false false))))))

(fn EventTrigger
  (params (IsPress :type Boolean))
  (switch Utilities|FlowControl|Switch|SwitchonEN_FC_Mode (Variables|Default|GetFC_Mode)
    (:NewEnumerator0
      (CallFunction|TriggerCreateMode IsPress))
    (:NewEnumerator1
      (CallFunction|TriggerDeleteMode IsPress))
    (:NewEnumerator2
      (CallFunction|TriggerMoveMode IsPress))
    (:NewEnumerator3
      (CallFunction|TriggerColorMode IsPress))))

(fn ChangeMode
  (params (FC_Mode :type EN_FC_Mode%20Enum :default "NewEnumerator0"))
  (Development|PrintString "FC Change Mode")
  (bind _output_get (Variables|Default|SetFC_Mode FC_Mode))
  (Default|CallEventDispatcherChangeMode _output_get))

(fn GetFurnitureObj
  (bind _widgetinteraction (Variables|Default|GetWidgetInteraction))
  (bind _returnvalue (Transformation|GetWorldLocation _widgetinteraction))
  (bind (_outhit _returnvalue_2) (Collision|LineTraceForObjects _returnvalue (+ _returnvalue (* (Math|Vector|GetForwardVector _widgetinteraction) (Variables|/Script/UMG.WidgetInteractionComponent|GetInteractionDistance _widgetinteraction))) (Utilities|Array|MakeArray "ObjectTypeQuery1" "ObjectTypeQuery2") false 0 "None"))
  (if _returnvalue_2
    (bind _asbp_furniture (Utilities|Casting|CastToBP_Furniture (.HitActor (Collision|BreakHitResult _outhit)))
      (:then
        (return _asbp_furniture))
      (:CastFailed
        _)))
  (return 0))

(fn IsShowFurniture
  (params (HitComponent :type Primitive%20Component%20Object%20Reference))
  (return (and (!= (Utilities|GetClass HitComponent) "/Script/UMG.WidgetComponent") (Utilities|Enum|Equal(Enum) (Variables|Default|GetFC_Mode) "NewEnumerator0"))))

(fn ChangeFurniture
  (bind _outrownames (DataTable|GetDataTableRowNames "/Game/ShowHouse/Data/DT_Furniture.DT_Furniture"))
  (bind _result (Math|Integer|IncrementInt (Variables|Default|GetCurFurnitureIndex))
    (:%20%20
      (if (>= _result (Utilities|Array|Length _outrownames))
        (Variables|Default|SetCurFurnitureIndex 0))
      (bind _output_get (Variables|Default|SetCurFurnitureRowName (Utilities|Array|Get(acopy) _outrownames (Variables|Default|GetCurFurnitureIndex))))
      (bind _returnvalue (Utilities|GetDataTableRow "/Game/ShowHouse/Data/DT_Furniture.DT_Furniture" _output_get)
        (:then
          (Components|StaticMesh|SetStaticMesh (Variables|Default|GetFurnitureMesh) (.StaticMesh (Utilities|Struct|BreakST_Furniture _returnvalue))))))))

(fn RotationFurniture
  (params (DeltaRotationZ :type Float%20%28double-precision%29))
  (bind _output_get (Variables|Default|SetOffsetRotationZ (+ DeltaRotationZ (Variables|Default|GetOffsetRotationZ))))
  (if (>= _output_get 3.6e+02)
    (Variables|Default|SetOffsetRotationZ 0.0)))

(fn TriggerCreateMode
  (params (IsPress :type Boolean))
  (if IsPress
    (Game|SpawnActorfromClass "/Game/ShowHouse/Blueprints/BP_Furniture.BP_Furniture_C" (Transformation|GetWorldTransform (Variables|Default|GetFurnitureMesh)) "Undefined" "MultiplyWithRoot" 0 (Variables|Default|GetCurFurnitureRowName) 0)))

(fn TriggerDeleteMode
  (params (IsPress :type Boolean))
  (bind _furniture (CallFunction|GetFurnitureObj))
  (if IsPress
    (Utilities|IsValid _furniture
      (:Is%20Valid
        (Actor|DestroyActor _furniture)))))

(fn TriggerMoveMode
  (params (IsPress :type Boolean))
  (bind _furniture (CallFunction|GetFurnitureObj))
  (if IsPress
    (Utilities|IsValid _furniture
      (:Is%20Valid
        (bind _output_get (Variables|Default|SetAttachFurniture _furniture))
        (Transformation|SetActorTransform _output_get (Math|Transform|MakeTransform "0, 0, 0"))
        (Collision|SetCollisionEnabled (Variables|/Game/ShowHouse/Blueprints/BP_Furniture.BP_Furniture_C|GetStaticMesh _output_get) "NoCollision")
        (Transformation|AttachComponentToComponent _output_get (Variables|Default|GetFurnitureMesh) "None" "KeepRelative" "KeepRelative" "KeepRelative" true)))
    (else
      (bind _attachfurniture (Variables|Default|GetAttachFurniture)
        (:then
          (Transformation|DetachFromActor _attachfurniture "KeepWorld" "KeepWorld" "KeepWorld")
          (Collision|SetCollisionEnabled (Variables|/Game/ShowHouse/Blueprints/BP_Furniture.BP_Furniture_C|GetStaticMesh _attachfurniture) "QueryAndPhysics")
          (Variables|Default|SetAttachFurniture 0))
        (:else)))))

(fn TriggerColorMode
  (params (IsPress :type Boolean))
  (bind _widgetinteraction (Variables|Default|GetWidgetInteraction))
  (bind _returnvalue (Transformation|GetWorldLocation _widgetinteraction))
  (if IsPress
    (bind (_outhit _returnvalue_2) (Collision|LineTraceForObjects _returnvalue (+ _returnvalue (* (Math|Vector|GetForwardVector _widgetinteraction) (Variables|/Script/UMG.WidgetInteractionComponent|GetInteractionDistance _widgetinteraction))) (Utilities|Array|MakeArray "ObjectTypeQuery2") false 0 "None"))
    (if _returnvalue_2
      (Utilities|IsValid (Actor|GetComponentbyClass (.HitActor (Collision|BreakHitResult _outhit)) "/Game/ShowHouse/Blueprints/MaterialListComponent.MaterialListComponent_C")
        (:Is%20Valid
          (Game|SpawnActorfromClass "/Game/ShowHouse/Blueprints/BP_PaletteActor.BP_PaletteActor_C" (Math|Transform|MakeTransform (+ (.Location (Collision|BreakHitResult _outhit)) (* (Math|Vector|GetForwardVector (Math|Rotator|FindLookatRotation (.Location (Collision|BreakHitResult _outhit)) (Transformation|GetActorLocation (Game|GetPlayerCameraManager 0)))) 5e+01)) "0, 0, 0" "1.000000,1.000000,1.000000") "Undefined" "MultiplyWithRoot" 0 (Actor|GetComponentbyClass (.HitActor (Collision|BreakHitResult _outhit)) "/Game/ShowHouse/Blueprints/MaterialListComponent.MaterialListComponent_C") 0))))))