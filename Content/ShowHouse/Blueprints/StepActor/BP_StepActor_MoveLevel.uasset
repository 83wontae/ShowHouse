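; A show house step actor that moves the player to another level.
; When the step starts, it fades the player camera out over five seconds and sets a timer by function name for the same duration.
; The timer calls the end-step override, which runs the parent logic and opens the level named by its LevelName variable.
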(event EventBeginPlay
  (|CallParentFunction) ; This node is disabled and will not be called.\nDrag off pins to build functionality.
)

(event Collision|EventActorBeginOverlap
  (params (OtherActor :type Actor%20Object%20Reference)))

(event EventTick
  (params (DeltaSeconds :type Float%20%28single-precision%29)))

(fn ConstructionScript
  (|CallParentFunction))

(fn EventStartStep
  (|CallParentFunction)
  (CameraFades|StartCameraFade :self (Game|GetPlayerCameraManager 0) :ToAlpha 1.0 :Duration 5.0)
  (Utilities|Time|SetTimerbyFunctionName 0 "EventEndStep" 5.0))

(fn EventEndStep
  (|CallParentFunction)
  (Game|OpenLevel(byName) (Variables|Default|GetLevel%20Name)))