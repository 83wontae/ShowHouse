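; Step actor that shows a titled popup widget with a description, with optional audio, for the duration of one step.
; BeginPlay hides the widget and fills in its text and sound.
; Starting the step reveals the popup and ends it when the audio finishes, or after a fixed timer if no sound is valid.
; Ending calls clear, which hides the widget, stops and unbinds the audio, and cancels any pending timer.
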(event EventBeginPlay
  (|CallParentFunction)
  (Rendering|SetVisibility (Variables|Default|GetWidget) false false)
  (bind _aspopup_widget (Utilities|Casting|CastToPopupWidget (UserInterface|GetUserWidgetObject (Variables|Default|GetWidget))))
  (Default|SetPopup _aspopup_widget (Variables|Default|GetTitle) (Variables|Default|GetDesc))
  (Audio|Components|Audio|SetSound (Variables|Default|GetAudio) (Variables|Default|GetSound)))

(fn ConstructionScript
  (|CallParentFunction))

(fn EventStartStep
  (|CallParentFunction)
  (Rendering|SetVisibility (Variables|Default|GetWidget) true false)
  (Variables|Default|GetSound
    (:then
      (EventDispatchers|BindEventtoOnAudioFinished (Variables|Default|GetAudio) (EventDispatchers|CreateEvent :!event EventAudioFinish))
      (Audio|Components|Audio|Play (Variables|Default|GetAudio) 0.0))
    (:else
      (Utilities|Time|SetTimerbyFunctionName 0 "EventEndStep" 5.0))))

(fn EventEndStep
  (|CallParentFunction)
  (CallFunction|EventClearStep))

(fn EventAudioFinish
  (CallFunction|EventEndStep))

(fn EventClearStep
  (bind _audio (Variables|Default|GetAudio))
  (|CallParentFunction)
  (Rendering|SetVisibility (Variables|Default|GetWidget) false false)
  (Utilities|FlowControl|Sequence
    (:then_0
      (EventDispatchers|UnbindallEventsfromOnAudioFinished _audio)
      (Audio|Components|Audio|Stop _audio))
    (:then_1
      (if (Class|KismetSystemLibrary|TimerExists 0 "EventEndStep")
        (Utilities|Time|ClearTimerbyFunctionName 0 "EventEndStep")))))