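; Step actor that teleports the player pawn to a target as one step in a step sequence, masked by a camera fade.
; Starting the step fades the camera out, then a timer calls DoTeleport to copy TeleportTarget's location and rotation onto the pawn and fade back in.
; A second timer ends the step after the fade-in, while clearing the step cancels only a pending teleport timer.
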(event EventBeginPlay
  (|CallParentFunction) ; This node is disabled and will not be called.\nDrag off pins to build functionality.
)

(event Collision|EventActorBeginOverlap
  (params (OtherActor :type Actor%20Object%20Reference)))

(event EventTick
  (params (DeltaSeconds :type Float%20%28single-precision%29)))

(fn ConstructionScript
  (|CallParentFunction))

(fn EventStartStep
  (|CallParentFunction)
  (CameraFades|StartCameraFade :self (Game|GetPlayerCameraManager 0) :ToAlpha 1.0 :Duration 5.0)
  (Utilities|Time|SetTimerbyFunctionName 0 "DoTeleport" 5.0))

(fn DoTeleport
  (bind _teleporttarget (Variables|Default|GetTeleportTarget))
  (Transformation|SetActorLocationAndRotation (Game|Player|GetPlayerPawn 0) (Transformation|GetActorLocation _teleporttarget) (Transformation|GetActorRotation _teleporttarget))
  (CameraFades|StartCameraFade :self (Game|GetPlayerCameraManager 0) :FromAlpha 1.0 :Duration 5.0)
  (Utilities|Time|SetTimerbyFunctionName 0 "EventEndStep" 5.0))

(fn EventClearStep
  (|CallParentFunction)
  (if (Class|KismetSystemLibrary|TimerExists 0 "DoTeleport")
    (Utilities|Time|ClearTimerbyFunctionName 0 "DoTeleport")))