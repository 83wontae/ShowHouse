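; BP_StepActor_Base is the base actor for one step in the ShowHouse content sequence, keyed to a MyStep content state.
; It binds to the game state's content-state dispatcher, starting when the state matches MyStep and calling an empty clear hook for other states, with one enum value ignored.
; Ending a step advances the game state to NextStep, chaining steps together.
; The construction script labels its TextRender with Comment or name and step.
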(event EventBeginPlay
  (bind _asbp_shgame_state (Utilities|Casting|CastToBP_SHGameState (Game|GetGameState)))
  (EventDispatchers|BindEventtoEventDispatcherContentState _asbp_shgame_state (EventDispatchers|CreateEvent :!event EventContentState)))

(fn ConstructionScript
  (bind _comment (Variables|Default|GetComment))
  (if (Utilities|Text|TextIsEmpty _comment)
    (Rendering|Components|TextRender|SetText (Variables|Default|GetTextRender) (Utilities|Text|ToText(String) (Utilities|String|Append (Utilities|GetDisplayName self) " - " (Utilities|String|EnumtoString (Variables|Default|GetMyStep)))))
    (else
      (Rendering|Components|TextRender|SetText (Variables|Default|GetTextRender) _comment))))

(fn EventContentState
  (params (ContentState :type EN_ContentState%20Enum :default "NewEnumerator3"))
  (bind _mystep (Variables|Default|GetMyStep))
  (if (Utilities|Enum|NotEqual(Enum) ContentState "NewEnumerator3")
    (if (Utilities|Enum|Equal(Enum) ContentState _mystep)
      (Development|PrintString (Utilities|String|Append (Utilities|GetDisplayName self) " - " (Utilities|String|EnumtoString _mystep)) true true "(R=0.000000,G=0.660000,B=1.000000,A=1.000000)" 2e+01)
      (CallFunction|EventStartStep)
      (else
        (CallFunction|EventClearStep)))))

(fn EventStartStep
  (Variables|Default|SetIsPlayingStep true))

(fn EventEndStep
  (Variables|Default|SetIsPlayingStep false)
  (bind _asbp_shgame_state (Utilities|Casting|CastToBP_SHGameState (Game|GetGameState)))
  (Default|ChangeContentState _asbp_shgame_state (Variables|Default|GetNextStep)))

(fn EventClearStep)