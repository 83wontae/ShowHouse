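; Step actor that fades the player's camera in as one step of a ShowHouse step sequence.
; On start, it prints the step name for debugging, starts a camera fade from full alpha and sets a timer that calls EventEndStep when the fade finishes.
; Clearing the step cancels that timer if it exists, and both overrides call their parent implementations first.
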(event EventBeginPlay
  (|CallParentFunction) ; This node is disabled and will not be called.\nDrag off pins to build functionality.
)

(event Collision|EventActorBeginOverlap
  (params (OtherActor :type Actor%20Object%20Reference)))

(event EventTick
  (params (DeltaSeconds :type Float%20%28single-precision%29)))

(fn ConstructionScript
  (|CallParentFunction))

(fn EventStartStep
  (|CallParentFunction)
  (Development|PrintString (Utilities|String|Append "EventStartStep - " (Utilities|String|EnumtoString (Variables|Default|GetMyStep))) true true "(R=0.000000,G=0.660000,B=1.000000,A=1.000000)" 6e+01)
  (CameraFades|StartCameraFade :self (Game|GetPlayerCameraManager 0) :FromAlpha 1.0 :Duration 5.0)
  (Utilities|Time|SetTimerbyFunctionName 0 "EventEndStep" 5.0))

(fn EventClearStep
  (|CallParentFunction)
  (if (Class|KismetSystemLibrary|TimerExists 0 "EventEndStep")
    (Utilities|Time|ClearTimerbyFunctionName 0 "EventEndStep")))