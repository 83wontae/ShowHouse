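; A show-house step actor that has the player select it by clicking in order to finish the step.
; Starting the step enables selection on BP_SHPawn and turns on the Box collision, and a click ends it.
; Clearing the step while it is playing switches both back off.
; Line overlap events show and hide the Decal as a highlight.
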(event EventBeginPlay
  (|CallParentFunction) ; This node is disabled and will not be called.\nDrag off pins to build functionality.
)

(event Collision|EventActorBeginOverlap
  (params (OtherActor :type Actor%20Object%20Reference)))

(event EventTick
  (params (DeltaSeconds :type Float%20%28single-precision%29)))

(fn ConstructionScript
  (|CallParentFunction))

(fn EventBeginOverlapLine
  (Rendering|SetVisibility (Variables|Default|GetDecal) true false))

(fn EventEndOverlapLine
  (Rendering|SetVisibility (Variables|Default|GetDecal) false false))

(fn EventStartStep
  (|CallParentFunction)
  (bind _asbp_shpawn (Utilities|Casting|CastToBP_SHPawn (Game|Player|GetPlayerPawn 0)))
  (Default|EnableSelect _asbp_shpawn true)
  (Collision|SetCollisionEnabled (Variables|Default|GetBox) "QueryAndPhysics"))

(fn EventEndStep
  (|CallParentFunction)
  (CallFunction|EventClearStep))

(fn EventClearStep
  (|CallParentFunction)
  (if (Variables|Default|GetIsPlayingStep)
    (bind _asbp_shpawn (Utilities|Casting|CastToBP_SHPawn (Game|Player|GetPlayerPawn 0)))
    (Default|EnableSelect _asbp_shpawn false)
    (Collision|SetCollisionEnabled (Variables|Default|GetBox) "NoCollision")
    (Variables|Default|SetIsPlayingStep false)))

(fn EventClick
  (CallFunction|EventEndStep)
  (return true))